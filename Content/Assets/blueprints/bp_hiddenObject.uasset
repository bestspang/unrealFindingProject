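; Hidden object Blueprint for a VR game that the player can pick up and drop, and that destroys itself when popped.
; Fake objects get a random material color at BeginPlay, when all objects bind to the VR pawn's pop event.
; Pickup and drop toggle physics, hand attachment and the pawn's IsGrab flag.
; Popping destroys the actor after a short delay; the particle and sound effects are disconnected.
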(event Custom|popped
  (Utilities|Casting|CastTobp_MyVRPawn (Game|Player|GetPlayerPawn 0))
  (if true
    (Utilities|FlowControl|Delay 0.1))
  (Actor|DestroyActor))

(event EventDropOff
  (bind _hiddenmesh (Variables|Default|GethiddenMesh))
  ;[0.2499 1 0.3458] Pickup and Drop
  (Physics|SetSimulatePhysics _hiddenmesh true)
  (Transformation|DetachFromComponent _hiddenmesh "KeepWorld" "KeepWorld" "KeepWorld" false)
  (bind _asbp_my_vrpawn (Utilities|Casting|CastTobp_MyVRPawn (Game|Player|GetPlayerPawn 0)))
  (Variables|/Game/Assets/player/bp_MyVRPawn.bp_MyVRPawn_C|SetisGrab _asbp_my_vrpawn false))

(event EventBeginPlay
  (Utilities|FlowControl|Sequence
    (:then_0
      (Variables|Default|SetcolorArray (Utilities|Array|MakeArray "0.000000,0.000000, 0" "0.000000,1.000000, 0" "0, 0,1.000000" "1.000000,1.000000, 0" "0,1.000000,1.000000" "1.000000, 0,1.000000" "1.000000,1.000000,1.000000")))
    (:then_1
      (if (Variables|Default|GetisFake)
        (Rendering|Material|SetVectorParameterValueonMaterials (Variables|Default|GethiddenMesh) "colorBase" (Utilities|Array|Get(acopy) (Variables|Default|GetcolorArray) (Math|Random|RandomIntegerinRange 0 (- (Utilities|Array|Length (Variables|Default|GetcolorArray)) 1))))))
    (:then_2
      (bind _outactors (Actor|GetAllActorsOfClass "/Game/Assets/player/bp_MyVRPawn.bp_MyVRPawn_C"))
      (bind _output_get (Variables|Default|SetmyVRPawn (Utilities|Array|Get(acopy) _outactors)))
      (EventDispatchers|BindEventtoPopHiddenObjects _output_get (delegate Custom|popped)))))

(event EventPickUp
  (params (ActorToAttachTo :type Scene%20Component%20Object%20Reference))
  ;[0.2499 1 0.3458] Pickup and Drop
  (Physics|SetSimulatePhysics (Variables|Default|GethiddenMesh) false)
  (Transformation|AttachComponentToComponent (VehicleSound|GetRootComponent) ActorToAttachTo "hand_LSocket" "KeepWorld" "KeepWorld" "KeepWorld" false)
  (bind _asbp_my_vrpawn (Utilities|Casting|CastTobp_MyVRPawn (Game|Player|GetPlayerPawn 0)))
  (Variables|/Game/Assets/player/bp_MyVRPawn.bp_MyVRPawn_C|SetisGrab _asbp_my_vrpawn true))

(fn ConstructionScript)