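; Score bucket actor for a VR game that awards a point when a hidden object enters its ScoreBox.
; On spawn it plays a click, adds a delayed particle emitter and binds its destroy event to the VR pawn's pop-bucket event for resets.
; An overlapping hidden object updates the pawn's counts, triggers normal, fire and fake respawns, and gets popped, then the bucket destroys itself and its emitter.
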(event OnComponentBeginOverlap(scoreBox)
  (params (OverlappedComponent :type Primitive%20Component%20Object%20Reference) (OtherActor :type Actor%20Object%20Reference) (OtherComp :type Primitive%20Component%20Object%20Reference) (OtherBodyIndex :type Integer) (bFromSweep :type Boolean) (SweepResult :type Hit%20Result%20Structure%20%28by%20ref%29))
  ;[1 0.07549 0.5918] Destroy actor when hit by Hidden object
  (if (== (Utilities|GetClass OtherActor) "/Game/Assets/blueprints/bp_hiddenObject.bp_hiddenObject_C")
    (CallFunction|AddPoint)
    (bind _asbp_hidden_object (Utilities|Casting|CastTobp_hiddenObject OtherActor))
    (Default|Popped _asbp_hidden_object)
    (CallFunction|DestroyBucket)))

(event Custom|destroyBucket
  ;[0.3012 1 0.107] binding - prepare for reset
  (Utilities|FlowControl|Delay 0.1)
  (Components|DestroyComponent (stale EventBeginPlay _returnvalue_2))
  (Actor|DestroyActor))

(event Custom|addPoint
  ;[1 0.5247 0.06714] add point
  (bind _asbp_my_vrpawn (Utilities|Casting|CastTobp_MyVRPawn (Game|Player|GetPlayerPawn 0)))
  (bind _result (Math|Integer|IncrementInt (Variables|/Game/Assets/player/bp_MyVRPawn.bp_MyVRPawn_C|GetScoreCount _asbp_my_vrpawn))
    (:%20%20
      (Math|Integer|DecrementInt (Variables|/Game/Assets/player/bp_MyVRPawn.bp_MyVRPawn_C|GetFireCount _asbp_my_vrpawn)
        (:%20%20
          (Variables|/Game/Assets/player/bp_MyVRPawn.bp_MyVRPawn_C|SetfinalCount _asbp_my_vrpawn _result)
          (Default|SpawnHiddenObject _asbp_my_vrpawn false false)
          (Default|SpawnHiddenObject _asbp_my_vrpawn false true 1 1)
          (Default|SpawnHiddenObject _asbp_my_vrpawn true false 1 3))))))

(event EventBeginPlay
  (bind _scorebox (Variables|Default|GetscoreBox))
  (bind _returnvalue (Transformation|GetWorldLocation _scorebox))
  ;[1 1 1] spawn emitter
  (Audio|PlaySoundatLocation "/Engine/VREditor/Sounds/VR_click1_Cue.VR_click1_Cue" _returnvalue)
  (Utilities|FlowControl|Delay 2.0)
  (bind _returnvalue_2 (Effects|SpawnEmitteratLocation "/Engine/Tutorial/SubEditors/TutorialAssets/TutorialParticleSystem.TutorialParticleSystem" _returnvalue))
  ;[0.3012 1 0.107] binding - prepare for reset
  (bind _outactors (Actor|GetAllActorsOfClass "/Game/Assets/player/bp_MyVRPawn.bp_MyVRPawn_C"))
  (bind _output_get (Variables|Default|SetMyVRPawn (Utilities|Array|Get(acopy) _outactors)))
  (EventDispatchers|BindEventtoPopBucket _output_get (delegate Custom|destroyBucket)))

(fn ConstructionScript)